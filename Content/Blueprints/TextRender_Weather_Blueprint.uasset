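; Text render Blueprint that displays the current weather description for Manhattan, fetched from the OpenWeatherMap web API.
; BeginPlay holds a VaRest GET call with a hardcoded URL and API key, though its request setup is marked disabled.
; The Response callback reads the first entry of the weather array and sets its description as the TextRender text.
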(event `self.ReceiveBeginPlay`
  (bind _returnvalue (subsystem `VaRestSubsystem`))
  (bind _returnvalue_2 (`VaRestSubsystem.ConstructVaRestJsonObject` _returnvalue :!enabledstate Disabled))
  (`VaRestSubsystem.CallURL` _returnvalue "http://api.openweathermap.org/data/2.5/weather?q=Manhattan&appid=5869d90bbf13ee5217d93f6779bcf236" "GET" "x_www_form_urlencoded_url" _returnvalue_2 (delegate `Response`)))

(event `Response`
  (params (Request :type "VaRestRequestJSON Object Reference"))
  (bind _returnvalue (`VaRestJsonValue.AsObject` (`|GetArrayItem` (`VaRestJsonObject.GetArrayField` (`VaRestRequestJSON.GetResponseObject` Request) "weather"))))
  (`TextRenderComponent.K2_SetText` (`self.TextRender`) (`KismetTextLibrary.Conv_StringToText` (`VaRestJsonObject.GetStringField` _returnvalue "description"))))

(fn `UserConstructionScript`)