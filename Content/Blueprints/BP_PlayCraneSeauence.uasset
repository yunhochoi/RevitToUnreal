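; Blueprint actor that plays the crane Level Sequence when the game starts.
; BeginPlay creates a sequence player for LevelSequence_Crain, plays it, then binds OnPlay and OnFinished events, whose handlers are empty.
; Tick prints the player's current playback time to screen as a debug readout.
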(event `self.ReceiveBeginPlay`
  (bind (_outactor _returnvalue) (`LevelSequencePlayer.CreateLevelSequencePlayer` "/Game/Sequences/LevelSequence_Crain.LevelSequence_Crain"))
  (`MovieSceneSequencePlayer.Play` _returnvalue)
  (add `MovieSceneSequencePlayer.OnPlay` _returnvalue (delegate `OnStarted`))
  (add `MovieSceneSequencePlayer.OnFinished` _returnvalue (delegate `OnFinished`)))

(event `OnStarted`)

(event `OnFinished`)

(event `self.ReceiveTick`
  (params (DeltaSeconds :type "Float (single-precision)"))
  (`KismetSystemLibrary.PrintString` (`KismetStringLibrary.TimeSecondsToString` (`TimeManagementBlueprintLibrary.Conv_QualifiedFrameTimeToSeconds` (`MovieSceneSequencePlayer.GetCurrentTime` (stale `self.ReceiveBeginPlay` _returnvalue))))))

(fn `UserConstructionScript`)