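; Example actor for a Socket.IO chat window, linking a chat widget component to a SocketIOClient.
; On BeginPlay it registers itself as the widget's message emitter and binds the chat event to ReceiveChatMessage, which forwards incoming text to the chat box.
; EmitChatMessage sends text to the server; M sends a test message and Enter focuses the widget.
; A generic-event handler shows an alternative receive style, but its binding is unwired.
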(event `self.ReceiveBeginPlay`
  (`self.SetupWidgetLinks`)
  (`SocketIOClientComponent.BindEventToFunction` (`self.SocketIOClient`) (`self.ChatEventName`) "ReceiveChatMessage" null "/" "USE_DEFAULT") ; bind event to a bp function
)

(event `Key|Enter`
  (params (Key :type "Key Structure"))
  (:`Pressed`
    (`Widget.SetKeyboardFocus` (`WidgetComponent.GetUserWidgetObject` (`self.ChatWidget`))) ; this should allow you to type
    (`KismetSystemLibrary.PrintString` "change focus to widget" false)))

(event `Key|M`
  (params (Key :type "Key Structure"))
  (:`Pressed`
    (`SocketIOClientComponent.Emit` (`self.SocketIOClient`) (`self.ChatEventName`) (`SIOJLibrary.Conv_StringToJsonValue` "hello socketio ue4!") "/")
    (`KismetSystemLibrary.PrintString` "pressed m" false)))

(event `self.SocketIOClient.OnGenericEvent`
  (params (EventName :type String) (MessageJson :type "SIOJsonValue Object Reference"))
  (if (`KismetStringLibrary.EqualEqual_StrStr` EventName (`self.ChatEventName`))
    (`self.MessageReceived` (`.ChatBoxWidget` (`self.ChatBoxWidget`)) (`SIOJsonValue.AsString` MessageJson))
    (`KismetSystemLibrary.PrintString` "event style message received" false) ; log it
    (else
      (`KismetSystemLibrary.PrintString` (`KismetStringLibrary.Concat_StrStr` "got unknown event: " EventName)) ; we got an unhandled event
    )))

(event `EmitChatMessage_1`
  (params (Message :type String))
  (`SocketIOClientComponent.Emit` (`self.SocketIOClient`) (`self.ChatEventName`) (`SIOJLibrary.Conv_StringToJsonValue` Message) "/"))

(fn `ReceiveChatMessage`
  (params (Message :type "SIOJsonValue Object Reference"))
  (`self.MessageReceived` (`.ChatBoxWidget` (`self.ChatBoxWidget`)) (`SIOJsonValue.AsString` Message)) ; received a message, forward it to the chat widget
  (`KismetSystemLibrary.PrintString` "function style message received" false) ; log it
)

(fn `SetupWidgetLinks`
  (bind _aschat_box_widget (cast `` (`WidgetComponent.GetUserWidgetObject` (`self.ChatWidget`))))
  (set `self.ChatBoxWidget` null _aschat_box_widget)
  (set `/Game/Blueprints/SocketIOExamples/ChatWindowActor.ChatMessageEmitter` self _aschat_box_widget))

(fn `UserConstructionScript`)